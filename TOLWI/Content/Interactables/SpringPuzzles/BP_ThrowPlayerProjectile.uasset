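; Projectile for the spring puzzles that stands in for the thrown small player and ends the throw when it hits something.
; On Hit it sets IsSmallThrown on MyTOLWIGameMode, calls ServerDeath on player controller 0, then destroys itself.
; A disconnected node that would spawn BP_SmallCharacter at the Sphere1 location never runs.
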(event Collision|EventHit
  (params (MyComp :type Primitive%20Component%20Object%20Reference) (Other :type Actor%20Object%20Reference) (OtherComp :type Primitive%20Component%20Object%20Reference) (bSelfMoved :type Boolean) (HitLocation :type Vector :default "0, 0, 0") (HitNormal :type Vector :default "0, 0, 0") (NormalImpulse :type Vector :default "0, 0, 0") (Hit :type Hit%20Result%20Structure%20%28by%20ref%29))
  (bind _asmy_tolwigame_mode (Utilities|Casting|CastToMyTOLWIGameMode (Game|GetGameMode)))
  (Variables|/Game/MyTOLWIGameMode.MyTOLWIGameMode_C|SetisSmallThrown? _asmy_tolwigame_mode true)
  (bind _asmy_tolwiplayer_controller (Utilities|Casting|CastToMyTOLWIPlayerController (Game|GetPlayerController 0)))
  (Default|ServerDeath _asmy_tolwiplayer_controller)
  (Actor|DestroyActor))

(fn ConstructionScript)