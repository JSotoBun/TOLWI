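; BP_Thorns is a spring puzzle interactable that slides a thorns mesh along a spline when activated.
; DoInteract calls Activate, which plays the Movement timeline and sets the mesh's world location at that fraction of the spline length, without sweep.
; BDoInteract always returns false.
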(event Custom|Activate
  (bind _movement (Timeline|Movement Play)
    (:Update
      (Transformation|SetWorldLocation (Variables|Default|GetStaticMesh) (Spline|GetLocationatDistanceAlongSpline (Variables|Default|GetSpline) (* _movement (Spline|GetSplineLength (Variables|Default|GetSpline))) "World") false false))))

(event EventDoInteract
  (CallFunction|Activate))

(fn ConstructionScript)

(fn BDoInteract
  (return false))