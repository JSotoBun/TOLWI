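; Pressure plate for a spring puzzle that responds to BP_BigCharacter overlapping its Box, despite the SmallChar in its name.
; Box overlap begin and end set the Activated flag and call DoInteract, which forwards to LargeMovePlatRef only while Activated is true.
; Stepping off therefore clears the flag without notifying the referenced platform, and bDoInteract always returns false.
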(event OnComponentBeginOverlap(Box)
  (params (OverlappedComponent :type Primitive%20Component%20Object%20Reference) (OtherActor :type Actor%20Object%20Reference) (OtherComp :type Primitive%20Component%20Object%20Reference) (OtherBodyIndex :type Integer) (bFromSweep :type Boolean) (SweepResult :type Hit%20Result%20Structure%20%28by%20ref%29))
  (Utilities|Casting|CastToBP_BigCharacter OtherActor)
  (Variables|Default|SetActivated? true)
  (Class|Interact|DoInteract))

(event OnComponentEndOverlap(Box)
  (params (OverlappedComponent :type Primitive%20Component%20Object%20Reference) (OtherActor :type Actor%20Object%20Reference) (OtherComp :type Primitive%20Component%20Object%20Reference) (OtherBodyIndex :type Integer))
  (Utilities|Casting|CastToBP_BigCharacter OtherActor)
  (Variables|Default|SetActivated? false)
  (Class|Interact|DoInteract))

(event EventBeginPlay)

(event Collision|EventActorBeginOverlap
  (params (OtherActor :type Actor%20Object%20Reference)))

(event EventTick
  (params (DeltaSeconds :type Float%20%28single-precision%29)))

(event EventDoInteract
  (if (Variables|Default|GetActivated?)
    (Default|DoInteract (Variables|Default|GetLargeMovePlatRef))))

(fn ConstructionScript)

(fn BDoInteract
  (return false))