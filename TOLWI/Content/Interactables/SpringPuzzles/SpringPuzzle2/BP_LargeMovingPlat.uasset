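; BP_LargeMovingPlat is an interactable moving platform from the spring puzzle set that slides its static mesh along a spline.
; Interacting toggles IsActivated, then after a configurable delay plays or reverses the Movement timeline, whose value positions the mesh by distance along the spline.
; In automatic mode, finishing a run flips the state and reactivates, so the platform shuttles back and forth.
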(event Custom|Activate
  (Utilities|FlowControl|Delay (Variables|Default|GetAutomaticDelay))
  (if (Variables|Default|GetisActivated?)
    (bind _direct (Timeline|Movement Play)
      (:Update
        (Transformation|SetWorldLocation (Variables|Default|GetStaticMesh) (Spline|GetLocationatDistanceAlongSpline (Variables|Default|GetSpline) (* _direct (Spline|GetSplineLength (Variables|Default|GetSpline))) "World") false false))
      (:Finished
        (if (Variables|Default|GetIsAutomatic?)
          (if (Variables|Default|GetIsActivated?)
            (Variables|Default|SetIsActivated? false)
            (else
              (Variables|Default|SetIsActivated? true)))
          (CallFunction|Activate))))
    (else
      (Timeline|Movement Reverse))))

(event EventBeginPlay)

(event Collision|EventActorBeginOverlap
  (params (OtherActor :type Actor%20Object%20Reference)))

(event EventTick
  (params (DeltaSeconds :type Float%20%28single-precision%29)))

(event EventDoInteract
  (if (Variables|Default|GetisActivated?)
    (Variables|Default|SetisActivated? false)
    (else
      (Variables|Default|SetisActivated? true)))
  (CallFunction|Activate))

(fn ConstructionScript)

(fn BDoInteract
  (return false))