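; BP_BigCharacter is the big character, which interacts with actors and throws picked-up boxes or the small character.
; Holding AimThrow opens a Tick gate that previews the arc with gravity-based debug line-trace segments, stopping and clamping control pitch on a hit.
; Throw input launches a box projectile.
; ThrowCharacter, not called here, destroys the small character and launches a player projectile, using the preview's launch velocity.
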(event EventBeginPlay)

(event Collision|EventActorBeginOverlap
  (params (OtherActor :type Actor%20Object%20Reference)))

(event EventTick
  (params (DeltaSeconds :type Float%20%28single-precision%29))
  (bind _returnvalue (Game|GetPlayerController 0))
  (bind _returnvalue_2 (Pawn|GetControlRotation _returnvalue :!class /Script/Engine.Controller))
  (Utilities|FlowControl|Sequence
    (:then_0
      (Utilities|FlowControl|Gate true
        (:Exit
          (if (Variables|Default|GetPickedUpPlayer)
            (CallFunction|DrawThrowTrajectory (Variables|Default|GetPlayerInitialLocalVelocity))
            (Variables|Default|SetOldRotation (Transformation|GetActorRotation))
            (Transformation|SetActorRotation (Math|Rotator|MakeRotator (.roll _returnvalue_2) (Math|Float|ClampAngle (.pitch _returnvalue_2) 0.0 0.0) (.yaw _returnvalue_2)))
            (else
              (CallFunction|DrawThrowTrajectory (Variables|Default|GetBoxInitialLocalVelocity)))))))))

(event Input|ActionEvents|InputActionAimThrow
  (params (Key :type Key%20Structure :default "None"))
  (bind _returnvalue (Game|GetPlayerController 0))
  (bind _returnvalue_2 (Pawn|GetControlRotation _returnvalue :!class /Script/Engine.Controller))
  (:Pressed
    (Utilities|FlowControl|Gate true) ; enters at Open
  )
  (:Released
    (Utilities|FlowControl|Gate true) ; enters at Close
  ))

(event Input|ActionEvents|InputActionInteract
  (params (Key :type Key%20Structure :default "None"))
  (:Pressed
    (if (Variables|Default|GetCanInteract)
      (Class|Interact|DoInteract(Message) (Variables|Default|GetInteractActor)))))

(event Input|ActionEvents|InputActionThrow
  (params (Key :type Key%20Structure :default "None"))
  (:Pressed
    (if (not (Variables|Default|GetPickedUpPlayer))
      (if (Variables|Default|GetPickedUpBox)
        (CallFunction|ThrowBox)
        (Variables|Default|SetPickedUpBox false)))))

(fn ConstructionScript)

(fn GetSegmentatTime
  (params (StartLocation :type Vector) (InitialVelocity :type Vector) (Gravity :type Vector) (Time1 :type Float%20%28single-precision%29) (Time2 :type Float%20%28single-precision%29))
  (return (+ StartLocation (* InitialVelocity Time1) (* Gravity (* Time1 Time1 0.5))) (+ StartLocation (* InitialVelocity Time2) (* Gravity (* Time2 Time2 0.5)))))

(fn DrawThrowTrajectory
  (params (VectorType :type Vector))
  (bind _returnvalue (Pawn|GetController))
  (bind _returnvalue_2 (Pawn|GetControlRotation :!class /Script/Engine.Pawn))
  (bind _sphere (Variables|Default|GetSphere))
  (bind _returnvalue_3 (Transformation|GetWorldLocation _sphere))
  (bind _returnvalue_4 (Math|Vector|RotateVector "0, 0, 0" _returnvalue_2))
  (bind _returnvalue_5 (Pawn|GetControlRotation _returnvalue :!class /Script/Engine.Controller))
  (bind _returnvalue_6 (+ _returnvalue_3 _returnvalue_4))
  (Variables|Default|SetStartLocation _returnvalue_6)
  (Variables|Default|SetInitialVelocity (Math|Transform|TransformDirection (Math|Transform|MakeTransform _returnvalue_6 _returnvalue_2) VectorType))
  (bind _index (Utilities|FlowControl|ForLoopwithBreak 0 (Math|Float|Floor (/ (Variables|Default|GetPathLifeTime) (Variables|Default|GetTimeInterval))))
    (:LoopBody
      (bind (_point1 _point2) (CallFunction|GetSegmentatTime (Variables|Default|GetStartLocation) (Variables|Default|GetInitialVelocity) "0, 0,-980.000000" (* _index (Variables|Default|GetTimeInterval)) (* (+ _index 1) (Variables|Default|GetTimeInterval))))
      (bind _returnvalue_7 (Collision|LineTraceByChannel _point1 _point2 "TraceTypeQuery1" true 0 "ForOneFrame"))
      (if _returnvalue_7
        (Pawn|SetControlRotation _returnvalue (Math|Rotator|MakeRotator (.roll _returnvalue_5) (Math|Float|ClampAngle (.pitch _returnvalue_5) -45.0 45.0) (.yaw _returnvalue_5)))
        (return)))))

(fn ThrowBox
  (bind _returnvalue (Pawn|GetControlRotation :!class /Script/Engine.Pawn))
  (bind _returnvalue_2 (Game|SpawnActorfromClass "/Game/Interactables/SpringPuzzles/SpringPuzzle2/BP_ThrowableBoxProjectile.BP_ThrowableBoxProjectile_C" (select false "" (Math|Transform|MakeTransform (+ (Transformation|GetWorldLocation (Variables|Default|GetSphere)) (Math|Vector|RotateVector "0, 0, 0" _returnvalue)) _returnvalue "2.000000,2.000000,2.000000")) "AdjustIfPossibleButDontSpawnIfColliding" 0 0)) ; Spawn projectile
  (Game|Components|ProjectileMovement|SetVelocityinLocalSpace (Variables|/Game/Interactables/SpringPuzzles/SpringPuzzle2/BP_ThrowableBoxProjectile.BP_ThrowableBoxProjectile_C|GetProjectileMovement _returnvalue_2) (Variables|Default|GetBoxInitialLocalVelocity))
  (return))

(fn GetReadytoThrow)

(fn DisableMovement)

(fn EnableMovement)

(fn PunchButtonPushed)

(fn GetSmallCharRef
  (bind _outactors (Actor|GetAllActorsOfClass "/Game/Characters/BP_SmallCharacter.BP_SmallCharacter_C"))
  (Variables|Default|SetSmallCharRef (Utilities|Array|Get(acopy) _outactors)))

(fn UpdateInteract
  (params (Interact%20Actor :type Actor%20Object%20Reference) (Can%20Interact? :type Boolean))
  (Variables|Default|SetInteractActor Interact%20Actor)
  (Variables|Default|SetCanInteract Can%20Interact?))

(fn ThrowCharacter
  (bind _returnvalue (Pawn|GetControlRotation :!class /Script/Engine.Pawn))
  (bind _outactors (Actor|GetAllActorsOfClass "/Game/Characters/BP_SmallCharacter.BP_SmallCharacter_C"))
  (Actor|DestroyActor _outactors)
  (bind _returnvalue_2 (Game|SpawnActorfromClass "/Game/Interactables/SpringPuzzles/BP_ThrowPlayerProjectile.BP_ThrowPlayerProjectile_C" (select false "" (Math|Transform|MakeTransform (+ (Transformation|GetWorldLocation (Variables|Default|GetSphere)) (Math|Vector|RotateVector "0, 0, 0" _returnvalue)) _returnvalue)) "AdjustIfPossibleButDontSpawnIfColliding" 0 0)) ; Spawn projectile
  (Game|Components|ProjectileMovement|SetVelocityinLocalSpace (Variables|/Game/Interactables/SpringPuzzles/BP_ThrowPlayerProjectile.BP_ThrowPlayerProjectile_C|GetProjectile _returnvalue_2) (Variables|Default|GetPlayerInitialLocalVelocity))
  (return))