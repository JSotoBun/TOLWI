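; BP_SmallCharacter is a character Blueprint that feeds jump, fall, landing and push states to its Little_AnimBP animation Blueprint.
; BeginPlay caches the anim instance, and Tick watches CharacterMovement falling transitions to set or clear IsLanding.
; Jump input sets IsJumping and cancels pushing.
; Holding Interact sets IsPushing unless the character is jumping or falling, and releasing it clears the flag.
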(event EventBeginPlay
  ;[1 1 1] Prepare reference to Little's animation blueprint
  (bind _aslittle_anim_bp (Utilities|Casting|CastToLittle_AnimBP (Components|SkeletalMesh|GetAnimInstance (Variables|Character|GetMesh))))
  (Variables|Default|SetLittleAnimBP _aslittle_anim_bp))

(event Collision|EventActorBeginOverlap
  (params (OtherActor :type Actor%20Object%20Reference)))

(event EventTick
  (params (DeltaSeconds :type Float%20%28single-precision%29))
  (if (AI|Components|NavMovement|IsFalling (Variables|Character|GetCharacterMovement))
    (Variables|Default|SetbIsFalling true)
    (bind _littleanimbp (Variables|Default|GetLittleAnimBP)
      (:then
        (Variables|/Game/Animations/Little/Little_AnimBP.Little_AnimBP_C|SetbIsLanding _littleanimbp false))
      (:else))
    (elif (Variables|Default|GetbIsFalling)
      (Variables|Default|SetbIsFalling false)
      (bind _littleanimbp_2 (Variables|Default|GetLittleAnimBP)
        (:then
          (Variables|/Game/Animations/Little/Little_AnimBP.Little_AnimBP_C|SetbIsLanding _littleanimbp_2 true))
        (:else)))))

(event Input|ActionEvents|InputActionJump
  (params (Key :type Key%20Structure :default "None"))
  (:Pressed
    (bind _littleanimbp (Variables|Default|GetLittleAnimBP)
      (:then
        (Variables|/Game/Animations/Little/Little_AnimBP.Little_AnimBP_C|SetbIsJumping _littleanimbp true)
        (Variables|/Game/Animations/Little/Little_AnimBP.Little_AnimBP_C|SetbIsPushing _littleanimbp false))
      (:else))))

(event Input|ActionEvents|InputActionInteract
  (params (Key :type Key%20Structure :default "None"))
  (:Pressed
    (CallFunction|InteractionPressed))
  (:Released
    (CallFunction|InteractionReleased)))

(fn ConstructionScript)

(fn InteractionPressed
  (bind _littleanimbp (Variables|Default|GetLittleAnimBP)
    (:then
      (if (and (not (Variables|/Game/Animations/Little/Little_AnimBP.Little_AnimBP_C|GetbIsJumping _littleanimbp)) (not (Variables|Default|GetbIsFalling)))
        (Variables|/Game/Animations/Little/Little_AnimBP.Little_AnimBP_C|SetbIsPushing (Variables|Default|GetLittleAnimBP) true)))
    (:else)))

(fn InteractionReleased
  (bind _littleanimbp (Variables|Default|GetLittleAnimBP)
    (:then
      (Variables|/Game/Animations/Little/Little_AnimBP.Little_AnimBP_C|SetbIsPushing _littleanimbp false))
    (:else)))